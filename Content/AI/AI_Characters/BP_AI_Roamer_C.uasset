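; Roamer AI Blueprint that acquires a player target through AI Perception.
; On perception updates, if the Blackboard's target actor is invalid, it scans updated actors for ones whose instigator controller is a player controller.
; Each match is written to the target key, so the last one wins; sensing success is not checked.
; A valid target is never replaced or cleared here.
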(event `self.AIPerception.OnPerceptionUpdated`
  (params (UpdatedActors :type "Array of Actor Object Reference (by ref)"))
  (`/Engine/EditorBlueprintResources/StandardMacros.IsValid` (`BlackboardComponent.GetValueAsObject` (`AIBlueprintHelperLibrary.GetBlackboard` null) (`self.TargetActor_KeyName`))
    (:`Is Not Valid`
      (for _array_element UpdatedActors
        (if (`Controller.IsPlayerController` (`self.GetInstigatorController` _array_element))
          (`BlackboardComponent.SetValueAsObject` (`AIBlueprintHelperLibrary.GetBlackboard` null) (`self.TargetActor_KeyName`) _array_element))))))

(fn `UserConstructionScript`
  (`parent.UserConstructionScript`))
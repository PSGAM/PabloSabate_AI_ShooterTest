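; Waiter AI character Blueprint, a thin child class that relies on its parent for its behavior.
; On BeginPlay it runs the parent logic, then applies its WALKSPEED value through ChangeMaxWalkSpeed.
; The walk-speed interface event, ChangeMaxWalkSpeed and the construction script only forward to the parent; Tick and overlap events are disabled.
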(event `self.ReceiveBeginPlay`
  (`parent.ReceiveBeginPlay`)
  (`self.ChangeMaxWalkSpeed` (`self.WALK_SPEED`)))

(event `/Game/AI/Interfaces/BPI_AI_Character.BPI_SetMaxWalkSpeed`
  (params (NewMaxWalkSpeed :type "Float (double-precision)"))
  (`parent.BPI_SetMaxWalkSpeed` NewMaxWalkSpeed))

(fn `ChangeMaxWalkSpeed`
  (params (NewMaxWalkSpeed :type "Float (double-precision)"))
  (`parent.ChangeMaxWalkSpeed` NewMaxWalkSpeed))

(fn `UserConstructionScript`
  (`parent.UserConstructionScript`))
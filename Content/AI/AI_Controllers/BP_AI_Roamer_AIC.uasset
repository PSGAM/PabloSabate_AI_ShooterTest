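; AI controller for a roaming enemy that runs the BT_Roamer behavior tree on its pawn and enables Tick once the pawn is valid.
; When perception senses a player-controlled character, it stores it as the target in the Blackboard and turns on rotate-and-strafe flags through an interface event.
; While rotation is on, Tick smoothly yaws the pawn toward the target.
; Losing perception does not clear the target.
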(event `self.ReceiveBeginPlay`
  (bind _returnvalue (`self.K2_GetPawn`))
  (`parent.ReceiveBeginPlay`)
  (`/Engine/EditorBlueprintResources/StandardMacros.IsValid` _returnvalue
    (:`Is Valid`
      (set `self.OwnersCharacter` _returnvalue)
      (`self.RunBehaviorTree` "/Game/AI/BehaviorTrees_And_BlackBoards/BT_Roamer.BT_Roamer")
      ;[0.3 1 0.3 0.3] if all is good enable the Tick
      (`self.SetActorTickEnabled` true))
    (:`Is Not Valid`
      (`KismetSystemLibrary.PrintString` (`KismetStringLibrary.Concat_StrStr` "[010523a] - GetControlledPawn failed in " (`KismetSystemLibrary.GetDisplayName` self)) true true (struct :`R` 1.0 :`A` 1.0) 10.0))))

(event `self.ReceiveTick`
  (params (DeltaSeconds :type "Float (single-precision)"))
  (bind _returnvalue (`self.K2_GetActorRotation` (`self.OwnersCharacter`)))
  ;[0.3 1 1 0.3] Tick - Will not execute if previously [OwnersCharacter] is not set at [BeginPlay]
  (if (`self.bUpdateRotation`)
    (`self.K2_SetActorRotation` (`self.OwnersCharacter`) (`KismetMathLibrary.RInterpTo` _returnvalue (`KismetMathLibrary.MakeRotator` (.roll _returnvalue) (.pitch _returnvalue) (.yaw (`KismetMathLibrary.FindLookAtRotation` (`self.K2_GetActorLocation` (`self.OwnersCharacter`)) (`self.K2_GetActorLocation` (`self.TargetActor`))))) (`GameplayStatics.GetWorldDeltaSeconds`) 5.0) false)))

(event `self.AIPerception.OnTargetPerceptionUpdated`
  (params (Actor :type "Actor Object Reference") (Stimulus :type "AIStimulus Structure"))
  (bind _ascharacter (cast `Character` Actor))
  (if (and (`Pawn.IsPlayerControlled` _ascharacter) (`.bSuccessfullySensed` (break `AIStimulus` Stimulus)))
    (set `self.TargetActor` Actor)
    (`BlackboardComponent.SetValueAsObject` (`self.Blackboard`) (`self.TargetActor_KeyName`) (`self.TargetActor`))
    (`self.BPI_RotateTowardsTarget` true)))

(event `self.BPI_RotateTowardsTarget`
  (params (`ShouldRotateTowardsTarget?` :type Boolean))
  (set `self.bUpdateRotation` `ShouldRotateTowardsTarget?`)
  (set `self.bAllowStrafe` `ShouldRotateTowardsTarget?`))

(fn `UserConstructionScript`
  (`parent.UserConstructionScript`))
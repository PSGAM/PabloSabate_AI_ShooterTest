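; AI controller for the waiter enemy that runs its behavior tree and reacts when perception senses the player.
; A sighting plays a get-up montage, switching the anim instance to combat on blend out and setting the blackboard target on completion.
; Completion also enables strafing and a Tick-driven, yaw-only interpolated turn toward the target through an interface event.
; Tick is enabled only if BeginPlay finds a valid pawn.
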(event `self.ReceiveBeginPlay`
  (bind _returnvalue (`self.K2_GetPawn`))
  (`parent.ReceiveBeginPlay`)
  (`/Engine/EditorBlueprintResources/StandardMacros.IsValid` _returnvalue
    (:`Is Valid`
      (set `self.OwnersPawn` _returnvalue)
      (`self.RunBehaviorTree` "/Game/AI/BehaviorTrees_And_BlackBoards/BT_Waiter.BT_Waiter")
      ;[0.3 1 0.3 0.3] if all is good enable the Tick
      (`self.SetActorTickEnabled` true))
    (:`Is Not Valid`
      (`KismetSystemLibrary.PrintString` (`KismetStringLibrary.Concat_StrStr` "[010523a] - GetControlledPawn failed in " (`KismetSystemLibrary.GetDisplayName` self)) true true (struct :`R` 1.0 :`A` 1.0) 10.0))))

(event `self.ReceiveTick`
  (params (DeltaSeconds :type "Float (single-precision)"))
  (bind _returnvalue (`self.K2_GetActorRotation` (`self.OwnersPawn`)))
  ;[0.3 1 1 0.3] Tick - Will not execute if previously [OwnersCharacter] is not set at [BeginPlay]
  (if (`self.bUpdateRotation`)
    (`self.K2_SetActorRotation` (`self.OwnersPawn`) (`KismetMathLibrary.RInterpTo` _returnvalue (`KismetMathLibrary.MakeRotator` (.roll _returnvalue) (.pitch _returnvalue) (.yaw (`KismetMathLibrary.FindLookAtRotation` (`self.K2_GetActorLocation` (`self.OwnersPawn`)) (`self.K2_GetActorLocation` (`self.TargetActor`))))) (`GameplayStatics.GetWorldDeltaSeconds`) 5.0) false)))

(event `self.AIPerception.OnTargetPerceptionUpdated`
  (params (Actor :type "Actor Object Reference") (Stimulus :type "AIStimulus Structure"))
  (bind _ascharacter (cast `Character` Actor))
  (if (and (`Pawn.IsPlayerControlled` _ascharacter) (`.bSuccessfullySensed` (break `AIStimulus` Stimulus)))
    (set `self.TargetActor` Actor)
    (bind _ascharacter_2 (cast `Character` (`self.OwnersPawn`)))
    (`|PlayMontage` (`Character.Mesh` _ascharacter_2) "/Game/AI/AnimationRelated/RM_GetUp_AM.RM_GetUp_AM"
      (:`OnCompleted`
        (`BlackboardComponent.SetValueAsObject` (`self.Blackboard`) (`self.TargetActor_KeyName`) (`self.TargetActor`))
        (`self.BPI_RotateTowardsTarget` true))
      (:`OnBlendOut`
        (bind _ascharacter_3 (cast `Character` (`self.OwnersPawn`)))
        (message `/Game/AI/AnimationRelated/AnimBPI_MasterAI.AnimBPI_SetInCombat` (`SkeletalMeshComponent.GetAnimInstance` (`Character.Mesh` _ascharacter_3)) true)))))

(event `self.BPI_RotateTowardsTarget`
  (params (`ShouldRotateTowardsTarget?` :type Boolean))
  (set `self.bUpdateRotation` `ShouldRotateTowardsTarget?`)
  (set `self.bAllowStrafe` `ShouldRotateTowardsTarget?`))

(fn `UserConstructionScript`
  (`parent.UserConstructionScript`))